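; BP_Tile is a grid tile actor that shows its status and power level and handles mouse interaction.
; Cursor hover darkens the top and, like clicks, notifies DefaultPlayerController, with the status material restored on exit.
; Status drives the top material or hides the mesh when destroyed, while Enable and Disable toggle visibility and collision.
; Power intensity only rises until reset, switching a second material slot between blue and black.
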(event `self.ReceiveBeginPlay`
  ;[1 1 1] TODO
  (`self.Enable`))

(event `self.ReceiveActorBeginCursorOver`
  ;[1 1 1] Mouse Interaction
  (`PrimitiveComponent.SetMaterial` (`self.TileMesh`) 0 "/Game/Assets/M_Black.M_Black")
  (bind _asdefault_player_controller (cast `/Game/Core/Game/Player/DefaultPlayerController` (`GameplayStatics.GetPlayerController` 0)))
  (`/Game/Core/Game/Player/DefaultPlayerController.TileHovered` _asdefault_player_controller self))

(event `self.ReceiveActorEndCursorOver`
  ;[1 1 1] Mouse Interaction
  (`self.SetTileTopMaterialFromStatus`))

(event `self.ReceiveActorOnClicked`
  (params (ButtonPressed :type "Key Structure"))
  ;[1 1 1] Mouse Interaction
  (bind _asdefault_player_controller (cast `/Game/Core/Game/Player/DefaultPlayerController` (`GameplayStatics.GetPlayerController` 0)))
  (`/Game/Core/Game/Player/DefaultPlayerController.TileClicked` _asdefault_player_controller self))

(fn `DebugTile`
  (returns (NewParam :type String))
  (return (`KismetStringLibrary.Concat_StrStr` "Y:" (`KismetStringLibrary.Conv_IntToString` (`self.YPos`)) " X: " (`KismetStringLibrary.Conv_IntToString` (`self.XPos`)))))

(fn `Disable`
  (`self.SetActorHiddenInGame` true)
  (`PrimitiveComponent.SetCollisionProfileName` (`self.TileMesh`) "NoCollision"))

(fn `Enable`
  (`self.SetActorHiddenInGame` false)
  (`PrimitiveComponent.SetCollisionProfileName` (`self.TileMesh`) "TiledObject"))

(fn `ResetPowerIntensity`
  (set `self.PowerIntensity` 0)
  (`PrimitiveComponent.SetMaterial` (`self.TileMesh`) 1 "/Game/Assets/M_Black.M_Black"))

(fn `SetPowerIntensity`
  (params (NewValue :type Integer))
  (returns (`DidUpdate?` :type Boolean))
  (if (> NewValue (`self.PowerIntensity`))
    (bind _output_get (set `self.PowerIntensity` NewValue))
    (`PrimitiveComponent.SetMaterial` (`self.TileMesh`) 1 "/Game/Assets/M_Blue.M_Blue")
    (return true)
    (else
      (return false))))

(fn `SetTileStatus`
  (params (Status :type "/Game/Core/Grid/ENUM_TileStatus Enum" :default "NewEnumerator0"))
  (bind _output_get (set `self.Status` Status))
  (switch `/Game/Core/Grid/ENUM_TileStatus` _output_get
    (:`NewEnumerator0`
      (`self.SetTileTopMaterialFromStatus` :!label _label))
    (:`NewEnumerator5`
      (`SceneComponent.SetVisibility` (`self.TileMesh`) false false))
    (:`NewEnumerator3`
      (goto _label))
    (:`NewEnumerator2`
      (goto _label))
    (:`NewEnumerator4`
      (goto _label))
    (:`NewEnumerator1`
      (goto _label))))

(fn `SetTileTopMaterialFromStatus`
  (bind _tilemesh (`self.TileMesh`))
  (switch `/Game/Core/Grid/ENUM_TileStatus` (`self.Status`)
    (:`NewEnumerator0`
      (`PrimitiveComponent.SetMaterial` _tilemesh 0 "/Game/Assets/M_Black.M_Black" :!label _label))
    (:`NewEnumerator3`
      (goto _label))
    (:`NewEnumerator2`
      (`PrimitiveComponent.SetMaterial` _tilemesh 0 "/Game/Assets/M_Red.M_Red"))
    (:`NewEnumerator4`
      (goto _label))
    (:`NewEnumerator1`
      (`PrimitiveComponent.SetMaterial` _tilemesh 0 "/Game/Assets/M_Blank.M_Blank"))))

(fn `UserConstructionScript`)