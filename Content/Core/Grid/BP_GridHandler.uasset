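; Grid manager that spawns an offset, hex-style BP_Tile map on BeginPlay and registers it with the player controller.
; Procedural passes place the core, spawn points and resources, optionally cut a circle, randomly destroy tiles and swap others for slow or speed tiles.
; Neighbor lookup on the flat tile array feeds recursive, decaying power propagation from generators and A*-style pathfinding through empty and checkpoint tiles.
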(event `self.ReceiveBeginPlay`
  (bind _tiles (`self.Tiles`))
  (`self.Spawn_Tiles`)
  (set `self.BaseDistance` (`KismetMathLibrary.FTrunc` (`self.GetDistanceTo` (`|GetArrayItem` _tiles) (`|GetArrayItem` _tiles 1))))
  (bind _asdefault_player_controller (cast `/Game/Core/Game/Player/DefaultPlayerController` (`GameplayStatics.GetPlayerController` 0)))
  (`/Game/Core/Game/Player/DefaultPlayerController.SetGrid` _asdefault_player_controller self)
  (`self.Procedural`)
  (if (> (`self.DestructionPercent`) 0)
    (`self.ProceduralDestruction`))
  (`self.ProceduralSpeedTiles`))

(fn `EndConstruction`)

(fn `FixRand`
  (params (Percent :type Integer))
  (returns (Ok :type Boolean))
  (return (>= Percent (`KismetMathLibrary.RandomIntegerInRange` 0 100))))

(fn `GetAdjacentTiles`
  (params (Tile :type "/Game/Core/Grid/BP_Tile Object Reference"))
  (returns (Tiles :type "Array of /Game/Core/Grid/BP_Tile Object Reference"))
  (locals (Result :type "Array of /Game/Core/Grid/BP_Tile Object Reference") (TileIndex :type Integer) (`XPosEven?` :type Boolean))
  (bind _tileindex (`local.TileIndex`))
  (bind _tiles (`self.Tiles`))
  (bind _result (`local.Result`))
  (bind _ypos (`/Game/Core/Grid/BP_Tile.YPos` Tile))
  (bind _tiles_2 (`self.Tiles`))
  (bind _result_2 (`local.Result`))
  (bind _tiles_3 (`self.Tiles`))
  (bind _result_3 (`local.Result`))
  (bind _ypos_2 (`/Game/Core/Grid/BP_Tile.YPos` Tile))
  (bind _tiles_4 (`self.Tiles`))
  (bind _result_4 (`local.Result`))
  (bind _xposeven_ (`local.XPosEven?`))
  (bind _result_5 (`local.Result`))
  (bind _ypos_3 (`/Game/Core/Grid/BP_Tile.YPos` Tile))
  (bind _tiles_5 (`self.Tiles`))
  (bind _returnvalue (- (`local.TileIndex`) (`self.Height`)))
  (bind _returnvalue_2 (+ (`local.TileIndex`) (`self.Height`)))
  (set `local.TileIndex` (`KismetArrayLibrary.Array_Find` (`self.Tiles`) Tile))
  (set `local.XPosEven?` (== (mod (`/Game/Core/Grid/BP_Tile.XPos` Tile) 2) 0))
  (`|ExecutionSequence`
    (:`then_0`
      (if (!= _ypos 0)
        (`KismetArrayLibrary.Array_Add` _result (`|GetArrayItem` _tiles (- _tileindex 1)))))
    (:`then_1`
      (if (!= _ypos (- (`self.Height`) 1))
        (`KismetArrayLibrary.Array_Add` _result (`|GetArrayItem` _tiles (+ _tileindex 1)))))
    (:`then_2`
      (if (!= (`/Game/Core/Grid/BP_Tile.XPos` Tile) 0)
        (if (!= _ypos_2 0)
          (if (`local.XPosEven?`)
            (`KismetArrayLibrary.Array_Add` _result_3 (`|GetArrayItem` _tiles_3 _returnvalue))
            (else
              (`KismetArrayLibrary.Array_Add` _result_3 (`|GetArrayItem` _tiles_3 (- _returnvalue 1))))))
        (if (!= _ypos_2 (- (`self.Height`) 1))
          (if (`local.XPosEven?`)
            (`KismetArrayLibrary.Array_Add` _result_2 (`|GetArrayItem` _tiles_2 (+ _returnvalue 1)))
            (else
              (`KismetArrayLibrary.Array_Add` _result_2 (`|GetArrayItem` _tiles_2 _returnvalue))))))
      (if (!= (`/Game/Core/Grid/BP_Tile.XPos` Tile) (- (`self.Width`) 1))
        (if (!= _ypos_3 0)
          (if _xposeven_
            (`KismetArrayLibrary.Array_Add` _result_4 (`|GetArrayItem` _tiles_4 _returnvalue_2))
            (`KismetArrayLibrary.Array_Add` _result_5 (`|GetArrayItem` _tiles_5 (+ _returnvalue_2 1)) :!label _label)
            (else
              (`KismetArrayLibrary.Array_Add` _result_4 (`|GetArrayItem` _tiles_4 (- _returnvalue_2 1)))
              (`KismetArrayLibrary.Array_Add` _result_5 (`|GetArrayItem` _tiles_5 _returnvalue_2) :!label _label_2)))
          (elif (!= _ypos_3 (- (`self.Height`) 1))
            (if _xposeven_
              (goto _label)
              (else
                (goto _label_2)))))))
    (:`then_3`
      (return (`local.Result`)))))

(fn `GetPathTo`
  (params (From :type "/Game/Core/Grid/BP_Tile Object Reference") (To :type "/Game/Core/Grid/BP_Tile Object Reference"))
  (returns (Path :type "Array of /Game/Core/Grid/BP_Tile Object Reference"))
  (locals (OpenList :type "Array of Integer") (CurrentEvaluatedIndex :type Integer) (Nodes :type "Map of Integer to /Game/Core/Grid/STRUCT_Pathfinding_Tile Structure") (Tmp :type "/Game/Core/Grid/STRUCT_Pathfinding_Tile Structure") (Rev_Result :type "Array of /Game/Core/Grid/BP_Tile Object Reference") (CloseList :type "Array of Integer") (Result :type "Array of /Game/Core/Grid/BP_Tile Object Reference") (`Inserted?` :type Boolean) (ParentEvaluatedIndex :type Integer))
  (bind _distance (`self.GetDistance` From To))
  (bind _nodes (`local.Nodes`))
  (bind _openlist (`local.OpenList`))
  (bind _currentevaluatedindex (`local.CurrentEvaluatedIndex`))
  (bind _rev_result (`local.Rev_Result`))
  (bind _openlist_2 (`local.OpenList`))
  (bind _result (`local.Result`))
  (bind _openlist_3 (`local.OpenList`))
  (bind _currentevaluatedindex_2 (`local.CurrentEvaluatedIndex`))
  (bind (_tile _parent _score _costfromstart) (break `/Game/Core/Grid/STRUCT_Pathfinding_Tile` (`local.Tmp`)))
  (bind (_tile_2 _parent_2) (break `/Game/Core/Grid/STRUCT_Pathfinding_Tile` (`local.Tmp`)))
  (bind _index (`self.GetIndexFromPos` (`/Game/Core/Grid/BP_Tile.YPos` From) (`/Game/Core/Grid/BP_Tile.XPos` From)))
  (bind (_tile_3 _parent_3 _score_2 _costfromstart_2 _distancetoend) (break `/Game/Core/Grid/STRUCT_Pathfinding_Tile` (`BlueprintMapLibrary.Map_Find` (`local.Nodes`) _currentevaluatedindex_2)))
  (bind _value (`BlueprintMapLibrary.Map_Find` (`local.Nodes`) _parent_2))
  (bind _value_2 (`BlueprintMapLibrary.Map_Find` (`local.Nodes`) (`|GetArrayItem` (`local.OpenList`))))
  (bind _returnvalue (+ _costfromstart 1))
  (bind _returnvalue_2 (+ (`.CostFromStart_10_2350FBB8400CC59FE6EF24A31FFEDBDF` (break `/Game/Core/Grid/STRUCT_Pathfinding_Tile` (`BlueprintMapLibrary.Map_Find` (`local.Nodes`) (`local.ParentEvaluatedIndex`)))) 1))
  (bind _returnvalue_3 (+ _distancetoend _returnvalue_2))
  ;[1 1 1] Init
  (`BlueprintMapLibrary.Map_Add` (`local.Nodes`) _index (make `/Game/Core/Grid/STRUCT_Pathfinding_Tile` From -1 _distance 0 _distance))
  (`KismetArrayLibrary.Array_Add` _openlist _index)
  (while (> (`KismetArrayLibrary.Array_Length` _openlist) 0)
    (set `local.Tmp` _value_2)
    (if (== (`local.To`) (`.Tile_2_ED832A964251B5ABE905B3A7A19F017F` (break `/Game/Core/Grid/STRUCT_Pathfinding_Tile` _value_2)))
      ;[1 1 1] Backtrack
      (`KismetArrayLibrary.Array_Add` _rev_result (`local.To`))
      (`KismetArrayLibrary.Array_Add` _rev_result _tile_2)
      (while (!= _parent_2 -1)
        (`KismetArrayLibrary.Array_Add` (`local.Rev_Result`) (`.Tile_2_ED832A964251B5ABE905B3A7A19F017F` (break `/Game/Core/Grid/STRUCT_Pathfinding_Tile` _value)))
        (set `local.Tmp` _value))
      (bind (_arrayindex _arrayelement) (`/Engine/EditorBlueprintResources/StandardMacros.ReverseForEachLoop` (`local.Rev_Result`))
        (:`LoopBody`
          (`KismetArrayLibrary.Array_Add` _result _arrayelement))
        (:`Completed`
          (return _result)))
      (else
        (`KismetArrayLibrary.Array_Add` (`local.CloseList`) (`|GetArrayItem` _openlist_3))
        (`KismetArrayLibrary.Array_Remove` _openlist_3)
        (set `local.ParentEvaluatedIndex` (`self.GetIndexFromPos` (`/Game/Core/Grid/BP_Tile.YPos` _tile) (`/Game/Core/Grid/BP_Tile.XPos` _tile)))
        (bind _tiles (`self.GetAdjacentTiles` _tile))
        (for _array_element _tiles
          (switch `/Game/Core/Grid/ENUM_TileStatus` (`/Game/Core/Grid/BP_Tile.Status` _array_element)
            (:`NewEnumerator3`
              _)
            (:`NewEnumerator1`
              _))
          (bind _output_get (set `local.CurrentEvaluatedIndex` (`self.GetIndexFromPos` (`/Game/Core/Grid/BP_Tile.YPos` _array_element) (`/Game/Core/Grid/BP_Tile.XPos` _array_element))))
          (if (not (!= (`KismetArrayLibrary.Array_Find` (`local.CloseList`) _output_get) -1))
            (bind _returnvalue_4 (`KismetArrayLibrary.Array_Find` (`local.OpenList`) _output_get))
            (if (!= _returnvalue_4 -1)
              ;[1 1 1] UpdateNode
              (if (> _costfromstart_2 _returnvalue_2)
                (`BlueprintMapLibrary.Map_Add` (`local.Nodes`) _currentevaluatedindex_2 (make `/Game/Core/Grid/STRUCT_Pathfinding_Tile` _tile_3 (`local.ParentEvaluatedIndex`) _returnvalue_3 _returnvalue_2 _distancetoend))
                (`KismetArrayLibrary.Array_Remove` (`local.OpenList`) _returnvalue_4)
                (for (_array_element_2 _array_index) _openlist_2
                  (if (> (`.Score_5_1CD9BFB04DB2779364B2EC803EF717F8` (break `/Game/Core/Grid/STRUCT_Pathfinding_Tile` (`BlueprintMapLibrary.Map_Find` (`local.Nodes`) _array_element_2))) _returnvalue_3)
                    (`KismetArrayLibrary.Array_Insert` _openlist_2 (`local.CurrentEvaluatedIndex`) _array_index)
                    (break))))
              (else
                (bind _distance_2 (`self.GetDistance` _array_element (`local.To`)))
                (bind _returnvalue_5 (+ _returnvalue _distance_2))
                (`BlueprintMapLibrary.Map_Add` _nodes (`local.CurrentEvaluatedIndex`) (make `/Game/Core/Grid/STRUCT_Pathfinding_Tile` _array_element (`local.ParentEvaluatedIndex`) _returnvalue_5 _returnvalue _distance_2))
                (`|ExecutionSequence`
                  (:`then_0`
                    (set `local.Inserted?` false))
                  (:`then_1`
                    (for (_array_element_3 _array_index_2) (`local.OpenList`)
                      (bind (_tile_4 _parent_4 _score_3 _costfromstart_3 _distancetoend_2) (break `/Game/Core/Grid/STRUCT_Pathfinding_Tile` (`BlueprintMapLibrary.Map_Find` _nodes _array_element_3)))
                      (if (or (> _score_3 _returnvalue_5) (and (== _score_3 _returnvalue_5) (> _distancetoend_2 _distance_2)))
                        (`KismetArrayLibrary.Array_Insert` (`local.OpenList`) _currentevaluatedindex _array_index_2)
                        (`|ExecutionSequence`
                          (:`then_0`
                            (set `local.Inserted?` true))
                          (:`then_1`
                            (break)))))
                    (if (not (`local.Inserted?`))
                      (`KismetArrayLibrary.Array_Add` (`local.OpenList`) _currentevaluatedindex)))))))))))
  (return))

(fn `Procedural`
  (locals (MaxDistance :type Integer :default 6) (CenterX :type Integer) (CenterY :type Integer) (Radius :type Integer))
  (bind _radius (`local.Radius`))
  (bind _tiles (`self.Tiles`))
  (bind _tiles_2 (`self.Tiles`))
  (bind _returnvalue (- (`self.Width`) 1))
  (bind _returnvalue_2 (/ (`self.Height`) 2))
  (bind _returnvalue_3 (- (`self.Height`) 1))
  (bind _returnvalue_4 (/ (`self.Height`) 2))
  (bind _returnvalue_5 (/ (`self.Width`) 2))
  (bind _returnvalue_6 (+ (/ _returnvalue 3) -1))
  (bind _returnvalue_7 (+ (/ _returnvalue_3 3) -1))
  (bind _returnvalue_8 (- _returnvalue_3 _returnvalue_7))
  (bind _returnvalue_9 (- _returnvalue _returnvalue_6))
  (cast `/Game/Core/Game/Player/DefaultPlayerController` (`GameplayStatics.GetPlayerController` 0))
  (`|ExecutionSequence`
    (:`then_0`
      ;[1 1 1] Core
      (`self.SimpleSpawn` "/Game/Core/Buildings/Core.Core_C" (`|GetArrayItem` (`self.Tiles`) (`self.GetIndexFromPos` _returnvalue_4 _returnvalue_5)))
      (set `local.CenterX` _returnvalue_5)
      (set `local.CenterY` _returnvalue_4))
    (:`then_1`
      ;[1 1 1] SpawnPoint
      (`self.SimpleSpawn` "/Game/Core/Buildings/SpawnPoint.SpawnPoint_C" (`|GetArrayItem` _tiles (`self.GetIndexFromPos` _returnvalue_2)))
      (`self.SimpleSpawn` "/Game/Core/Buildings/SpawnPoint.SpawnPoint_C" (`|GetArrayItem` _tiles (`self.GetIndexFromPos` _returnvalue_2 (- (`self.Width`) 1)))))
    (:`then_2`
      ;[1 1 1] Ressources
      (`self.SimpleSpawn` "/Game/Core/Buildings/DebugRessource.DebugRessource_C" (`|GetArrayItem` _tiles_2 (`self.GetIndexFromPos` _returnvalue_7 _returnvalue_6)))
      (`self.SimpleSpawn` "/Game/Core/Buildings/DebugRessource.DebugRessource_C" (`|GetArrayItem` _tiles_2 (`self.GetIndexFromPos` _returnvalue_7 _returnvalue_9)))
      (`self.SimpleSpawn` "/Game/Core/Buildings/DebugRessource.DebugRessource_C" (`|GetArrayItem` _tiles_2 (`self.GetIndexFromPos` _returnvalue_8 _returnvalue_9)))
      (`self.SimpleSpawn` "/Game/Core/Buildings/DebugRessource.DebugRessource_C" (`|GetArrayItem` _tiles_2 (`self.GetIndexFromPos` _returnvalue_8 _returnvalue_6))))
    (:`then_3`
      (switch `int` (`self.Shape`)
        (:`1`
          ;[1 1 1] Circle
          (set `local.Radius` (`local.CenterX`))
          (for _array_element (`self.Tiles`)
            (bind _returnvalue_10 (- (`/Game/Core/Grid/BP_Tile.XPos` _array_element) (`local.CenterX`)))
            (bind _returnvalue_11 (- (`/Game/Core/Grid/BP_Tile.YPos` _array_element) (`local.CenterY`)))
            (if (and (`|EnumEquality` (`/Game/Core/Grid/BP_Tile.Status` _array_element) "NewEnumerator1") (>= (+ (* _returnvalue_10 _returnvalue_10) (* _returnvalue_11 _returnvalue_11)) (* _radius _radius)))
              (`/Game/Core/Grid/BP_Tile.SetTileStatus` _array_element "NewEnumerator5"))))))))

(fn `ProceduralDestruction`
  (locals (TmpTiles :type "Array of /Game/Core/Grid/BP_Tile Object Reference"))
  (`KismetArrayLibrary.Array_Clear` (`local.TmpTiles`))
  (for _array_element (`self.Tiles`)
    (if (`|EnumEquality` (`/Game/Core/Grid/BP_Tile.Status` _array_element) "NewEnumerator1")
      (bind _yes_ (`self.ShouldDestroy?`))
      (if _yes_
        (`KismetArrayLibrary.Array_Add` (`local.TmpTiles`) _array_element)
        (`/Game/Core/Grid/BP_Tile.SetTileStatus` _array_element "NewEnumerator5")))))

(fn `ProceduralSpeedTiles`
  (locals (TmpTile :type "/Game/Core/Grid/BP_Tile Object Reference"))
  (for (_array_element _array_index) (`self.Tiles`)
    (if (`|EnumEquality` (`/Game/Core/Grid/BP_Tile.Status` _array_element) "NewEnumerator1")
      (bind _ok (`self.FixRand` (`self.SlowPercent`)))
      (if _ok
        (bind _output_get (set `local.TmpTile` _array_element))
        (bind _returnvalue (`|SpawnActorFromClass` "/Game/Core/Grid/Tile_MoveSpeed.Tile_MoveSpeed_C" (`self.GetTransform` _output_get) "Undefined" "OverrideRootScale" null (`/Game/Core/Grid/BP_Tile.XPos` _output_get) (`/Game/Core/Grid/BP_Tile.YPos` _output_get) null))
        (`/Game/Core/Grid/Tile_MoveSpeed.Init` _returnvalue -30.0)
        (`KismetArrayLibrary.Array_Set` (`self.Tiles`) _array_index _returnvalue)
        (`self.K2_DestroyActor` (`local.TmpTile`))
        (else
          (bind _ok_2 (`self.FixRand` (`self.SpeedPercent`)))
          (if _ok_2
            (bind _output_get_2 (set `local.TmpTile` _array_element))
            (bind _returnvalue_2 (`|SpawnActorFromClass` "/Game/Core/Grid/Tile_MoveSpeed.Tile_MoveSpeed_C" (`self.GetTransform` _output_get_2) "Undefined" "OverrideRootScale" null (`/Game/Core/Grid/BP_Tile.XPos` _output_get_2) (`/Game/Core/Grid/BP_Tile.YPos` _output_get_2) null))
            (`/Game/Core/Grid/Tile_MoveSpeed.Init` _returnvalue_2 30.0)
            (`KismetArrayLibrary.Array_Set` (`self.Tiles`) _array_index _returnvalue_2)
            (`self.K2_DestroyActor` (`local.TmpTile`))))))))

(fn `REC_UpdatePowerDistribution`
  (params (Tile :type "/Game/Core/Grid/BP_Tile Object Reference") (PowerIntensity :type Integer))
  (bind _didupdate_ (`/Game/Core/Grid/BP_Tile.SetPowerIntensity` Tile PowerIntensity))
  (if (and _didupdate_ (> PowerIntensity 0))
    (bind _tiles (`self.GetAdjacentTiles` Tile))
    (for _array_element _tiles
      (`self.REC_UpdatePowerDistribution` _array_element (- PowerIntensity 1)))))

(fn `ResetPowerDistribution`
  (for _array_element (`self.Tiles`)
    (`/Game/Core/Grid/BP_Tile.ResetPowerIntensity` _array_element)))

(fn `ShouldDestroy?`
  (returns (`Yes!` :type Boolean))
  (return (> (`self.DestructionPercent`) (`KismetMathLibrary.RandomIntegerInRange` 0 100))))

(fn `SimpleSpawn`
  (params (Class :type "Actor Class Reference") (Tile :type "/Game/Core/Grid/BP_Tile Object Reference"))
  (bind _returnvalue (`|SpawnActorFromClass` Class (`SceneComponent.K2_GetComponentToWorld` (`/Game/Core/Grid/BP_Tile.DefaultSceneRoot` Tile)) "Undefined" "OverrideRootScale" null null))
  (bind _asa_building (cast `/Game/Core/Buildings/A_Building` _returnvalue))
  (`KismetArrayLibrary.Array_Add` (`/Game/Core/Buildings/A_Building.OccupiedTiles` _asa_building) Tile)
  (`/Game/Core/Buildings/A_Building.DropBuildingInit` _asa_building))

(fn `Spawn_Tiles`
  (locals (Tile_W :type "Float (double-precision)" :default 200.0) (Tile_H :type "Float (double-precision)" :default 200.0) (LocationOffset :type "Vector Structure") (TileSize :type "Float (double-precision)" :default 200.0))
  (bind _tilesize (`local.TileSize`))
  (bind _z (.z (`local.LocationOffset`)))
  (bind _returnvalue (`KismetMathLibrary.MakeVector` 0.0 (`local.TileSize`)))
  (bind _returnvalue_2 (+ (.y (`local.LocationOffset`)) 27.0))
  (bind _returnvalue_3 (* (/ (`KismetMathLibrary.Conv_IntToDouble` (`self.Width`)) 2.0) (`local.TileSize`)))
  (`|ExecutionSequence`
    (:`then_0`
      ;[1 1 1] Init
      (set `local.LocationOffset` (`KismetMathLibrary.MakeVector` (* (/ (`KismetMathLibrary.Conv_IntToDouble` (`self.Width`)) 2.0) _tilesize) (* _tilesize (/ (`KismetMathLibrary.Conv_IntToDouble` (`self.Height`)) 2.0)))))
    (:`then_1`
      (for _index (range (`self.Width`))
        (for _index_2 (range (`self.Height`))
          (`|ExecutionSequence`
            (:`then_0`
              ;[1 1 1] SpawnTile
              (bind _returnvalue_4 (`|SpawnActorFromClass` "/Game/Core/Grid/BP_Tile.BP_Tile_C" (`KismetMathLibrary.MakeTransform` (+ (`local.LocationOffset`) (.location (`SceneComponent.K2_GetComponentToWorld` (`self.DefaultSceneRoot`)))) (.rotation (`SceneComponent.K2_GetComponentToWorld` (`self.DefaultSceneRoot`))) (.scale (`SceneComponent.K2_GetComponentToWorld` (`self.DefaultSceneRoot`)))) "Undefined" "OverrideRootScale" null _index _index_2 null))
              (`KismetArrayLibrary.Array_Add` (`self.Tiles`) _returnvalue_4)
              (`/Game/Core/Grid/BP_Tile.SetTileStatus` _returnvalue_4 "NewEnumerator1"))
            (:`then_1`
              ;[1 1 1] UpdateLocalOffset
              (set `local.LocationOffset` (- (`local.LocationOffset`) (`KismetMathLibrary.MakeVector` (`local.TileSize`)))))))
        ;[1 1 1] Update Offset
        (if (== (mod _index 2) 0)
          (set `local.LocationOffset` (- (`KismetMathLibrary.MakeVector` (+ _returnvalue_3 (/ (`local.TileSize`) 2.0)) _returnvalue_2 _z) _returnvalue))
          (else
            (set `local.LocationOffset` (- (`KismetMathLibrary.MakeVector` _returnvalue_3 _returnvalue_2 _z) _returnvalue))))))))

(fn `StartConstruction`)

(fn `UpdatePowerDistribution`
  (params (Generators :type "Array of /Game/Core/Buildings/A_Generator Object Reference"))
  (for _array_element Generators
    (for _array_element_2 (`/Game/Core/Buildings/A_Building.OccupiedTiles` _array_element)
      (`self.REC_UpdatePowerDistribution` _array_element_2 (`/Game/Core/Buildings/A_Generator.BaseIntensity` _array_element)))))

(fn `UserConstructionScript`
  (locals (Current :type "Transform Structure") (Tile_W :type "Float (double-precision)" :default 200.0) (Tile_H :type "Float (double-precision)" :default 230.0)))